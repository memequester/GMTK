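; Troop spawner that creates Infantry, Tank or Jeep units and charges their cost to the level's funds.
; SpawnTroop spawns the chosen class at the referenced spline track's transform, passes it that track, then deducts its cost without checking the balance and prints the remainder.
; BeginPlay caches LevelControl from the third-person game mode, then runs a test loop that spawns Infantry every five seconds via a custom event.
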(event `self.ReceiveBeginPlay`
  (`|ExecutionSequence`
    (:`then_0`
      ;[0.02083 0.02083 0.02083] Get Level Control Reference
      (bind _asbp_third_person_game_mode (cast `/Game/ThirdPerson/Blueprints/BP_ThirdPersonGameMode` (`GameplayStatics.GetGameMode`)))
      (set `self.LevelControlRef` (`/Game/ThirdPerson/Blueprints/BP_ThirdPersonGameMode.Level Control` _asbp_third_person_game_mode)))
    (:`then_1`
      ;[1 1 1] Test
      (`KismetSystemLibrary.Delay` 5.0 :!label _label)
      (`self.SpawnTroop` "NewEnumerator0")
      (`self.CustomEvent`))))

(event `CustomEvent`
  ;[1 1 1] Test
  (goto _label))

(fn `SpawnTroop`
  (params (TroopType :type "/Game/Troops/Enum_TroopType Enum" :default "NewEnumerator0"))
  (locals (SplineTransform :type "Transform Structure"))
  (bind _splinetransform (`local.SplineTransform`))
  (bind _splinetrackref (`self.SplineTrackRef`))
  (set `local.SplineTransform` (`self.GetTransform` (`self.SplineTrackRef`)))
  (switch `/Game/Troops/Enum_TroopType` (`local.TroopType`)
    (:`NewEnumerator0`
      (bind _returnvalue (`|SpawnActorFromClass` "/Game/Troops/BP_Troop_Infantry.BP_Troop_Infantry_C" _splinetransform "Undefined" "MultiplyWithRoot" null _splinetrackref null)))
    (:`NewEnumerator1`
      (bind _returnvalue_2 (`|SpawnActorFromClass` "/Game/Troops/BP_Troop_Tank.BP_Troop_Tank_C" _splinetransform "Undefined" "MultiplyWithRoot" null _splinetrackref null)))
    (:`NewEnumerator2`
      (bind _returnvalue_3 (`|SpawnActorFromClass` "/Game/Troops/BP_Troop_Jeep.BP_Troop_Jeep_C" _splinetransform "Undefined" "MultiplyWithRoot" null _splinetrackref null))))
  (bind _output_get (set `/Game/RonansCorner/Blueprints/Widgets/LevelControl.CurrentFunds` (- (`/Game/RonansCorner/Blueprints/Widgets/LevelControl.CurrentFunds` (`self.LevelControlRef`)) (`.Cost_19_930446AF4D8E2054163C089F19E82C50` (break `/Game/Data/Troop_Struct` (select `/Game/Troops/Enum_TroopType` (`local.TroopType`) :`NewEnumerator0` (`/Game/Troops/BP_Troop_Master.TroopData` _returnvalue) :`NewEnumerator1` (`/Game/Troops/BP_Troop_Master.TroopData` _returnvalue_2) :`NewEnumerator2` (`/Game/Troops/BP_Troop_Master.TroopData` _returnvalue_3))))) (`self.LevelControlRef`)))
  (`KismetSystemLibrary.PrintString` (`KismetStringLibrary.Conv_DoubleToString` _output_get)))

(fn `UserConstructionScript`)