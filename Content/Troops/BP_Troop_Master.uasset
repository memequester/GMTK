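; Base troop actor that travels along the spline of a referenced track from BeginPlay.
; The construction script loads the TroopData_DT row matching its troop type (Infantry, Tank or other) and scales the timeline play rate by speed over spline length.
; The TroopMovement timeline's alpha maps to distance along the spline, setting world location and rotation on each update.
; StartMovement and StopMovement events play and stop that timeline.
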(event `self.ReceiveBeginPlay`
  (`self.StartMovement`))

(event `StartMovement`
  ;[0.02083 0.02083 0.02083] Movement along Spline
  (bind (_direction _alpha) (`Timeline|TroopMovement` :!label _label)
    (:`Update`
      (`self.MoveTroop` _alpha))))

(event `StopMovement`
  ;[0.02083 0.02083 0.02083] Movement along Spline
  (goto _label :!via `Stop`))

(fn `GetSplineInfo`
  (returns (Spline :type "SplineComponent Object Reference") (Length :type "Float (single-precision)"))
  (bind _splinetrack (`/Game/SplineSystem/BP_SplineTrack.SplineTrack` (`self.TrackReference`)))
  (return _splinetrack (`SplineComponent.GetSplineLength` _splinetrack)))

(fn `MoveTroop`
  (params (Alpha :type "Float (single-precision)"))
  (bind (_spline _length) (`self.GetSplineInfo`))
  (bind _returnvalue (`KismetMathLibrary.Lerp` 0.0 _length (`local.Alpha`)))
  (`self.K2_SetActorLocationAndRotation` (`SplineComponent.GetLocationAtDistanceAlongSpline` _spline _returnvalue "World") (`SplineComponent.GetRotationAtDistanceAlongSpline` _spline _returnvalue "World")))

(fn `SetTroopSpeed`
  (`TimelineComponent.SetPlayRate` (`self.TroopMovement`) (/ (`.Speed_23_AB1C19C44D224FB402EF76A5EF4929F1` (break `/Game/Data/Troop_Struct` (`self.TroopData`))) (`.Length` (`self.GetSplineInfo`)) 0.1))
  (return))

(fn `UserConstructionScript`
  ;[0.02083 0.02083 0.02083] Get Troop Data and store as variable
  (bind _returnvalue (`|GetDataTableRow` "/Game/Data/TroopData_DT.TroopData_DT" (select `/Game/Troops/Enum_TroopType` (`self.TroopType`) :`NewEnumerator0` "Unit1" :`NewEnumerator1` "Unit2" :`NewEnumerator2` "Unit3" :!type "Name"))
    (:`then`
      (set `self.TroopData` _returnvalue)
      (`self.SetTroopSpeed`))))