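; BP_PlayerController is the player controller that turns Enhanced Input zoom, move and rotate actions into camera pawn controls.
; BeginPlay adds the default input mapping context to the local player subsystem.
; Each action runs through the UsingCameraPawn macro, which compares CurrentPawn to CameraPawnRef and calls the matching camera event only on the Camera branch.
; The macro's Troop branch is left unhandled, and neither pawn variable is set here.
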(event `self.ReceiveBeginPlay`
  (bind _returnvalue (subsystem `EnhancedInputLocalPlayerSubsystem`))
  (`|ExecutionSequence`
    (:`then_0`
      ;[0.02083 0.02083 0.02083] Add Mapping Context
      (`/Engine/EditorBlueprintResources/StandardMacros.IsValid` _returnvalue
        (:`Is Valid`
          (`EnhancedInputSubsystemInterface.AddMappingContext` _returnvalue "/Game/PlayerPawn/Input/IMC_Default.IMC_Default" 0 (struct)))))))

(event `EnhancedInput|/Game/PlayerPawn/Input/Actions/IA_Zoom`
  (params (ActionValue :type "Float (double-precision)") (ElapsedSeconds :type "Float (double-precision)") (TriggeredSeconds :type "Float (double-precision)") (InputAction :type "InputAction Object Reference" :default "/Game/PlayerPawn/Input/Actions/IA_Zoom.IA_Zoom"))
  (:`Triggered`
    (`self.UsingCameraPawn?`
      (:`Camera`
        (`/Game/PlayerPawn/Blueprints/BP_CameraPawn.EventCameraZoom` (`self.CameraPawnRef`) ActionValue)))))

(event `EnhancedInput|/Game/PlayerPawn/Input/Actions/IA_Move`
  (params (ActionValue :type "Vector2D Structure") (ElapsedSeconds :type "Float (double-precision)") (TriggeredSeconds :type "Float (double-precision)") (InputAction :type "InputAction Object Reference" :default "/Game/PlayerPawn/Input/Actions/IA_Move.IA_Move"))
  (bind (_x _y) (`KismetMathLibrary.BreakVector2D` ActionValue))
  (:`Triggered`
    (`self.UsingCameraPawn?`
      (:`Camera`
        (`/Game/PlayerPawn/Blueprints/BP_CameraPawn.EventCameraMove` (`self.CameraPawnRef`) _x _y)))))

(event `EnhancedInput|/Game/PlayerPawn/Input/Actions/IA_Rotate`
  (params (ActionValue :type "Float (double-precision)") (ElapsedSeconds :type "Float (double-precision)") (TriggeredSeconds :type "Float (double-precision)") (InputAction :type "InputAction Object Reference" :default "/Game/PlayerPawn/Input/Actions/IA_Rotate.IA_Rotate"))
  (:`Triggered`
    (`self.UsingCameraPawn?`
      (:`Camera`
        (`/Game/PlayerPawn/Blueprints/BP_CameraPawn.EventCameraRotate` (`self.CameraPawnRef`) ActionValue)))))

(fn `UserConstructionScript`)