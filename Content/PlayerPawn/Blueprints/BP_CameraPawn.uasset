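; BP_CameraPawn is a player camera pawn that pans, rotates and zooms with smoothed motion.
; On BeginPlay it exchanges references with BP_PlayerController and seeds the desired zoom and location from its current state.
; Camera events adjust desired targets, with pan relative to facing and both pan and zoom clamped.
; Tick interpolates boom length, actor location and rotation toward those targets.
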(event `self.ReceiveTick`
  (params (DeltaSeconds :type "Float (single-precision)"))
  ;[0.02083 0.02083 0.02083] Interpolate Camera Zoom
  (set `SpringArmComponent.TargetArmLength` (`KismetMathLibrary.FInterpTo` (`SpringArmComponent.TargetArmLength` (`self.CameraBoom`)) (`self.ZoomDesired`) DeltaSeconds 2.0) (`self.CameraBoom`))
  ;[0.02083 0.02083 0.02083] Interpolate Camera Location
  (`self.K2_SetActorLocation` (`KismetMathLibrary.VInterpTo` (`self.K2_GetActorLocation`) (`self.LocationDesired`) DeltaSeconds 2.0))
  (`self.K2_SetActorRotation` (`KismetMathLibrary.RInterpTo` (`self.K2_GetActorRotation`) (`self.RotateDesired`) DeltaSeconds 5.0)))

(event `self.ReceiveBeginPlay`
  (`|ExecutionSequence`
    (:`then_0`
      ;[0.02083 0.02083 0.02083] Set Controller References
      (bind _asbp_player_controller (cast `/Game/PlayerPawn/Blueprints/BP_PlayerController` (`GameplayStatics.GetPlayerController` 0)))
      (set `self.PlayerControllerRef` _asbp_player_controller)
      (bind _output_get (set `/Game/PlayerPawn/Blueprints/BP_PlayerController.CameraPawnRef` self _asbp_player_controller))
      (set `/Game/PlayerPawn/Blueprints/BP_PlayerController.CurrentPawn` _output_get (`self.PlayerControllerRef`)))
    (:`then_1`
      (set `self.ZoomDesired` (`SpringArmComponent.TargetArmLength` (`self.CameraBoom`)))
      (set `self.LocationDesired` (`self.K2_GetActorLocation`)))))

(event `EventCameraZoom`
  (params (ZoomValue :type "Float (double-precision)"))
  ;[0.02083 0.02083 0.02083] Camera Zoom Functionality
  (set `self.ZoomDesired` (`KismetMathLibrary.FClamp` (+ (`self.ZoomDesired`) (* ZoomValue (`self.ZoomMultiplier`))) (`self.ZoomMin`) (`self.ZoomMax`))))

(event `EventCameraMove`
  (params (Right :type "Float (double-precision)") (Forward :type "Float (double-precision)"))
  (bind _locationmultiplier (`self.LocationMultiplier`))
  (set `self.LocationDesired` (`/Game/Libraries/BPFunctionLibrary.ClampVector` (+ (`self.LocationDesired`) (+ (* (* Right _locationmultiplier) (`self.GetActorRightVector`)) (* (`self.GetActorForwardVector`) (* _locationmultiplier Forward)))) (`self.LocationMin`) (`self.LocationMax`))))

(event `EventCameraRotate`
  (params (RotateValue :type "Float (double-precision)"))
  (set `self.RotateDesired` (`KismetMathLibrary.ComposeRotators` (`self.RotateDesired`) (`KismetMathLibrary.MakeRotator` 0.0 0.0 (* RotateValue (`self.RotateMultiplier`))))))

(fn `UserConstructionScript`)