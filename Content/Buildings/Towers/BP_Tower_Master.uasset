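; Base tower that automatically targets and damages troops, with stats loaded from a data table row chosen by tower type in the construction script.
; Troops entering the range sphere trigger target search: Machine Gun picks nearest, Artillery highest health, Rocket furthest along by movement alpha.
; A self-calling delay loop applies damage at the fire rate and re-searches when the target is invalid, while Tick smoothly aims the weapon.
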(event `self.ReceiveTick`
  (params (DeltaSeconds :type "Float (single-precision)"))
  (bind _target (`self.Target`)
    (:`then`
      (`SceneComponent.K2_SetWorldRotation` (`self.Weapon`) (`KismetMathLibrary.RInterpTo` (`SceneComponent.K2_GetComponentRotation` (`self.Weapon`)) (`KismetMathLibrary.FindLookAtRotation` (`SceneComponent.K2_GetComponentLocation` (`self.Weapon`)) (`SceneComponent.K2_GetComponentLocation` (`/Game/Troops/BP_Troop_Master.DefaultSceneRoot` _target))) DeltaSeconds 3.0) false false))
    (:`else`)))

(event `StartAttacking`
  (`self.AttackTroops`)
  (`/Engine/EditorBlueprintResources/StandardMacros.IsValid` (`self.Target`)
    (:`Is Valid`
      (`KismetSystemLibrary.Delay` (`.RateofFire_24_F4B1AD14410CC1C9FC2E658C76F97E6D` (break `/Game/Data/Towers_Struct` (`self.TowerData`))))
      (`self.StartAttacking`))
    (:`Is Not Valid`
      (`KismetSystemLibrary.DelayUntilNextTick`)
      (`self.SearchForTarget`))))

(event `SearchForTarget`
  (`self.FindTarget`)
  (`self.StartAttacking`))

(event `self.MaxRange.OnComponentBeginOverlap`
  (params (OverlappedComponent :type "PrimitiveComponent Object Reference") (OtherActor :type "Actor Object Reference") (OtherComp :type "PrimitiveComponent Object Reference") (OtherBodyIndex :type Integer) (bFromSweep :type Boolean) (SweepResult :type "HitResult Structure (by ref)"))
  ;[0.02083 0.02083 0.02083] Search for Target when Troop enters range and Tower has no Target
  (cast `/Game/Troops/BP_Troop_Master` OtherActor)
  (`/Engine/EditorBlueprintResources/StandardMacros.IsValid` (`self.Target`)
    (:`Is Not Valid`
      (`self.SearchForTarget`))))

(event `self.MaxRange.OnComponentEndOverlap`
  (params (OverlappedComponent :type "PrimitiveComponent Object Reference") (OtherActor :type "Actor Object Reference") (OtherComp :type "PrimitiveComponent Object Reference") (OtherBodyIndex :type Integer))
  (if (== OtherActor (`self.Target`))
    (set `self.Target` null)))

(fn `AttackTroops`
  (bind ((`Damage_16_0B072DEB476964B22D81608DDF2B3B02` _damage)) (break `/Game/Data/Towers_Struct` (`self.TowerData`)))
  (bind _target (`self.Target`)
    (:`then`
      (bind _asbp_troop_master (cast `/Game/Troops/BP_Troop_Master` _target))
      (`/Game/Troops/BP_Troop_Master.TakeDamage` _asbp_troop_master _damage self)
      (`KismetSystemLibrary.PrintString` (`KismetStringLibrary.Conv_DoubleToString` _damage))
      (return))
    (:`else`)))

(fn `FindTarget`
  (switch `/Game/Buildings/Towers/Enum_Tower_Type` (`self.TowerType`)
    (:`NewEnumerator0`
      (`self.Nearest`))
    (:`NewEnumerator1`
      (`self.Strongest`))
    (:`NewEnumerator2`
      (`self.First`))))

(fn `First`
  (locals (BestAlpha :type "Float (double-precision)") (FirstTroop :type "/Game/Troops/BP_Troop_Master Object Reference"))
  (bind _overlappingactors (`PrimitiveComponent.GetOverlappingActors` (`self.MaxRange`) "/Game/Troops/BP_Troop_Master.BP_Troop_Master_C"))
  (set `local.FirstTroop` null)
  (if (`KismetArrayLibrary.Array_IsNotEmpty` _overlappingactors)
    (for _array_element _overlappingactors
      (bind _asbp_troop_master (cast `/Game/Troops/BP_Troop_Master` _array_element))
      (bind _firsttroop (`local.FirstTroop`)
        (:`then`
          (if (< (`/Game/Troops/BP_Troop_Master.MovementAlpha` _firsttroop) (`/Game/Troops/BP_Troop_Master.MovementAlpha` _asbp_troop_master))
            (set `local.FirstTroop` _asbp_troop_master :!label _label)))
        (:`else`
          (goto _label))))
    (bind _asbp_troop_master_2 (cast `/Game/Troops/BP_Troop_Master` (`local.FirstTroop`)))
    (set `self.Target` _asbp_troop_master_2)
    (return)
    (else
      (return))))

(fn `Nearest`
  (bind _overlappingactors (`PrimitiveComponent.GetOverlappingActors` (`self.MaxRange`) "/Game/Troops/BP_Troop_Master.BP_Troop_Master_C"))
  (if (`KismetArrayLibrary.Array_IsNotEmpty` _overlappingactors)
    (bind _asbp_troop_master (cast `/Game/Troops/BP_Troop_Master` (`.ReturnValue` (`GameplayStatics.FindNearestActor` (`SceneComponent.K2_GetComponentLocation` (`self.DefaultSceneRoot`)) _overlappingactors))))
    (set `self.Target` _asbp_troop_master)))

(fn `NormalizedHealth`
  (returns (NormalizedHealth :type "Float (double-precision)"))
  (return (/ (`self.CurrentHealth`) (`.MaxHealth_17_C4E8FE9446540B794F27B6BBD686CD5D` (break `/Game/Data/Towers_Struct` (`self.TowerData`))))))

(fn `Strongest`
  (locals (StrongestTroop :type "/Game/Troops/BP_Troop_Master Object Reference"))
  (set `local.StrongestTroop` null)
  (for _array_element (`PrimitiveComponent.GetOverlappingActors` (`self.MaxRange`) "/Game/Troops/BP_Troop_Master.BP_Troop_Master_C")
    (bind _asbp_troop_master (cast `/Game/Troops/BP_Troop_Master` _array_element))
    (bind _strongesttroop (`local.StrongestTroop`)
      (:`then`
        (if (> (`/Game/Troops/BP_Troop_Master.CurrentHealth` _asbp_troop_master) (`/Game/Troops/BP_Troop_Master.CurrentHealth` _strongesttroop))
          (set `local.StrongestTroop` _asbp_troop_master :!label _label)))
      (:`else`
        (goto _label))))
  (bind _asbp_troop_master_2 (cast `/Game/Troops/BP_Troop_Master` (`local.StrongestTroop`)))
  (set `self.Target` _asbp_troop_master_2)
  (return))

(fn `UserConstructionScript`
  (bind ((`MaxRange_18_C9C6C8654BCF33B748FB78A4CD24392F` _maxrange) (`MinRange_21_62FAA75743015F6146109F958A5EFD96` _minrange)) (break `/Game/Data/Towers_Struct` (`self.TowerData`)))
  (`|ExecutionSequence`
    (:`then_0`
      ;[0.02083 0.02083 0.02083] Set Tower Data from Data Table
      (bind _returnvalue (`|GetDataTableRow` "/Game/Data/TowersData_DT.TowersData_DT" (select `/Game/Buildings/Towers/Enum_Tower_Type` (`self.TowerType`) :`NewEnumerator0` "MachineGun" :`NewEnumerator1` "Artillery" :`NewEnumerator2` "Rocket" :!type "Name"))
        (:`then`
          (set `self.TowerData` _returnvalue))))
    (:`then_1`
      ;[0.02083 0.02083 0.02083] Set Current Health
      (set `self.CurrentHealth` (`.MaxHealth_17_C4E8FE9446540B794F27B6BBD686CD5D` (break `/Game/Data/Towers_Struct` (`self.TowerData`)))))
    (:`then_2`
      ;[0.02083 0.02083 0.02083] Set Min/Max Ranges
      (`SphereComponent.SetSphereRadius` (`self.MaxRange`) _maxrange true)
      (`SphereComponent.SetSphereRadius` (`self.MinRange`) _minrange true))))