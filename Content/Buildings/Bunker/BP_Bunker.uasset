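; BP_Bunker is the target building that troops attack, with sliding doors and health taken from LevelControl's level data.
; A troop overlapping the door trigger plays a timeline that slides both doors open, then a retriggerable delay rechecks until the area is clear and reverses it.
; Troops reaching the entry trigger subtract their bunker damage and are destroyed, and a win message prints when health runs out.
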(event `self.ReceiveBeginPlay`)

(event `self.DoorCollision.OnComponentBeginOverlap`
  (params (OverlappedComponent :type "PrimitiveComponent Object Reference") (OtherActor :type "Actor Object Reference") (OtherComp :type "PrimitiveComponent Object Reference") (OtherBodyIndex :type Integer) (bFromSweep :type Boolean) (SweepResult :type "HitResult Structure (by ref)"))
  ;[0.02083 0.02083 0.02083] Open Door upon actor being in area
  (cast `/Game/Troops/BP_Troop_Master` OtherActor)
  (bind (_direction _doorslide) (`Timeline|MoveDoor` :!label _label)
    (:`Update`
      (`SceneComponent.K2_SetRelativeLocation` (`self.Door L`) (`KismetMathLibrary.MakeVector` (`KismetMathLibrary.Lerp` 150.0 400.0 _doorslide) 300.0 60.0) false false)
      (`SceneComponent.K2_SetRelativeLocation` (`self.Door R`) (`KismetMathLibrary.MakeVector` (`KismetMathLibrary.Lerp` -150.0 -400.0 _doorslide) 300.0 60.0) false false))
    (:`Finished`
      (`self.DoorMovementFinished` _direction))))

(event `CloseDoors`
  ;[0.02083 0.02083 0.02083] Open Door upon actor being in area
  (goto _label :!via `Reverse`))

(event `DoorMovementFinished`
  (params (Direction :type "ETimelineDirection Enum" :default "Forward"))
  ;[0.02083 0.02083 0.02083] Open Door upon actor being in area
  (if (`|EnumEquality` Direction "Forward")
    (`KismetSystemLibrary.RetriggerableDelay` 1.5 :!label _label_2)
    (if (`KismetArrayLibrary.Array_IsEmpty` (`PrimitiveComponent.GetOverlappingActors` (`self.DoorCollision`) "/Game/Troops/BP_Troop_Master.BP_Troop_Master_C"))
      (`self.CloseDoors`)
      (else
        (goto _label_2)))))

(event `self.BunkerEntered.OnComponentBeginOverlap`
  (params (OverlappedComponent :type "PrimitiveComponent Object Reference") (OtherActor :type "Actor Object Reference") (OtherComp :type "PrimitiveComponent Object Reference") (OtherBodyIndex :type Integer) (bFromSweep :type Boolean) (SweepResult :type "HitResult Structure (by ref)"))
  (bind _asbp_troop_master (cast `/Game/Troops/BP_Troop_Master` OtherActor))
  (set `self.CurrentHealth` (- (`self.CurrentHealth`) (`.BunkerDamage_26_E06DAA104DE8A3094CD097B2E64BFF73` (break `/Game/Data/Troop_Struct` (`/Game/Troops/BP_Troop_Master.TroopData` _asbp_troop_master)))))
  (`self.K2_DestroyActor` _asbp_troop_master)
  (`self.CheckHealth`))

(event `CheckHealth`
  (bind _currenthealth (`self.CurrentHealth`))
  (if (<= _currenthealth 0.0)
    (`KismetSystemLibrary.PrintString` "YOU WIN!!")
    (else
      (`KismetSystemLibrary.PrintString` (`KismetStringLibrary.Conv_DoubleToString` _currenthealth)))))

(fn `TroopEntered`)

(fn `UserConstructionScript`
  (`|ExecutionSequence`
    (:`then_0`
      ;[0.02083 0.02083 0.02083] Reference for Control
      (bind _returnvalue (`GameplayStatics.GetActorOfClass` "/Game/RonansCorner/Blueprints/Widgets/LevelControl.LevelControl_C"))
      (set `self.LevelControlRef` _returnvalue))
    (:`then_1`
      ;[0.02083 0.02083 0.02083] Set Max Health
      (set `self.CurrentHealth` (`.BunkerMaxHealth_15_9B26F7994FEF835494BB7DA9DC19C064` (break `/Game/Data/LevelSizes/LevelData_DS` (`/Game/RonansCorner/Blueprints/Widgets/LevelControl.LevelData` (`self.LevelControlRef`))))))))