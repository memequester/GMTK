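; Bunker actor that slides its double doors apart when a troop approaches and removes troops that go inside.
; A door trigger plays the MoveDoor timeline, whose updates call MoveComponentTo on both doors, with no closing logic.
; An entry trigger destroys any overlapping BP_Troop_Master.
; LevelControl is cached on BeginPlay, but TroopEntered is empty and the construction script only assigns BunkerMaxHealth to itself.
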(event `self.DoorCollision.OnComponentBeginOverlap`
  (params (OverlappedComponent :type "PrimitiveComponent Object Reference") (OtherActor :type "Actor Object Reference") (OtherComp :type "PrimitiveComponent Object Reference") (OtherBodyIndex :type Integer) (bFromSweep :type Boolean) (SweepResult :type "HitResult Structure (by ref)"))
  ;[1 1 1] Open Door upon actor being in area
  (cast `/Game/Troops/BP_Troop_Master` OtherActor)
  (bind (_direction _door_r _door_l _doorslide) (`Timeline|MoveDoor`)
    (:`Update`
      (`KismetSystemLibrary.MoveComponentTo` (`self.Door L`) (400.0 300.0 0.0) (struct) false true _doorslide)
      (`KismetSystemLibrary.MoveComponentTo` (`self.Door R`) (-400.0 300.0 0.0) (struct) false true _doorslide))))

(event `self.BunkerEntered.OnComponentBeginOverlap`
  (params (OverlappedComponent :type "PrimitiveComponent Object Reference") (OtherActor :type "Actor Object Reference") (OtherComp :type "PrimitiveComponent Object Reference") (OtherBodyIndex :type Integer) (bFromSweep :type Boolean) (SweepResult :type "HitResult Structure (by ref)"))
  (bind _asbp_troop_master (cast `/Game/Troops/BP_Troop_Master` OtherActor))
  (`self.K2_DestroyActor` _asbp_troop_master))

(event `self.ReceiveBeginPlay`
  ;[1 1 1] Reference for Control
  (bind _returnvalue (`GameplayStatics.GetActorOfClass` "/Game/RonansCorner/Blueprints/Widgets/LevelControl.LevelControl_C"))
  (set `self.LevelControlRef` _returnvalue))

(fn `TroopEntered`)

(fn `UserConstructionScript`
  (bind _levelcontrolref (`self.LevelControlRef`))
  (set `/Game/RonansCorner/Blueprints/Widgets/LevelControl.BunkerMaxHealth` (`/Game/RonansCorner/Blueprints/Widgets/LevelControl.BunkerMaxHealth` _levelcontrolref) _levelcontrolref))